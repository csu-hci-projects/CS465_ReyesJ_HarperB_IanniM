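; Office room Blueprint that configures its desk computer meshes and plays a timed startup sound sequence on BeginPlay.
; It looks up the GlobalVariables actor and uses its UseHP flag to choose HP monitor, logo and keyboard-wire meshes or three computer-wire meshes, nudging the first into place.
; A UFO startup sound plays immediately, followed after roughly ten seconds by an old monitor power-on and degauss sound.
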(event EventBeginPlay
  (bind _returnvalue (Actor|GetActorOfClass "/Game/Globals/GlobalVariables.GlobalVariables_C"))
  (Variables|Default|SetGlobalVar _returnvalue)
  (CallFunction|SetDeskMesh)
  (Audio|PlaySoundatLocation "/Game/GameMechanics/Sounds/ufo-start-up-68712.ufo-start-up-68712" "0, 0, 0" "0, 0, 0" 1.0 1.0 0.0 0 0 0 0)
  (Utilities|FlowControl|Delay 9.9)
  (Audio|PlaySoundatLocation "/Game/GameMechanics/Sounds/old-pc-monitor-switch-on-and-degaussing-8576.old-pc-monitor-switch-on-and-degaussing-8576" "0, 0, 0" "0, 0, 0" 1.0 1.0 0.0 0 0 0 0))

(event Collision|EventActorBeginOverlap
  (params (OtherActor :type Actor%20Object%20Reference)))

(event EventTick
  (params (DeltaSeconds :type Float%20%28single-precision%29)))

(fn ConstructionScript)

(fn SetDeskMesh
  (bind _deskmesh1 (Variables|Default|GetDeskMesh1))
  (bind _deskmesh1_2 (Variables|Default|GetDeskMesh1))
  (bind _deskmesh2 (Variables|Default|GetDeskMesh2))
  (bind _deskmesh3 (Variables|Default|GetDeskMesh3))
  (if (Variables|/Game/Globals/GlobalVariables.GlobalVariables_C|GetUseHP (Variables|Default|GetGlobalVar))
    (Components|StaticMesh|SetStaticMesh _deskmesh1_2 "/Game/Computer/Types/LabComputer/Meshes/HPMonitor.HPMonitor")
    (Components|StaticMesh|SetStaticMesh _deskmesh2 "/Game/Computer/Types/LabComputer/Meshes/HPLogo.HPLogo")
    (Components|StaticMesh|SetStaticMesh _deskmesh3 "/Game/BlenderImports/OfficeRoom/Cables/Meshes/HPKeyboardWire.HPKeyboardWire")
    (Transformation|AddLocalOffset _deskmesh1 "4.000000,6.800000,0.000000" false false)
    (else
      (Components|StaticMesh|SetStaticMesh _deskmesh1_2 "/Game/BlenderImports/OfficeRoom/Cables/Meshes/ComputerWire3.ComputerWire3")
      (Components|StaticMesh|SetStaticMesh _deskmesh2 "/Game/BlenderImports/OfficeRoom/Cables/Meshes/ComputerWire2.ComputerWire2")
      (Components|StaticMesh|SetStaticMesh _deskmesh3 "/Game/BlenderImports/OfficeRoom/Cables/Meshes/ComputerWire1.ComputerWire1")
      (Transformation|AddLocalOffset _deskmesh1 "3.000000,1.000000,0.000000" false false))))