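; Computer actor for a typing experiment, with an animated keyboard and an on-screen text display.
; Validated key presses drive key animation and sound, repeat while held, and are converted for Shift, Caps Lock and symbols.
; Characters are checked against GlobalVariables' prompt and coloured on the task monitor.
; Each finished task stores WPM, accuracy and a keystroke log, then the next prompt loads or data is saved and input disabled.
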(event Custom|Pressed
  (params (KeyName :type String) (KeyIndex :type Integer))
  ;[1 1 1 1 34] Key Pressed: Checks that the input given is safe for manipulation and display
  (bind _output_get (Variables|Default|SetCurrentKey KeyName))
  (Utilities|InsertKeyinLiveClicks _output_get
    (:TrackingKey
      ;;[0.1559 0.1559 0.1559 1 12] Set the visual offset of the key on the keyboard
      (CallFunction|SetKeyAnimation KeyIndex true)
      ;;[0.1559 0.1559 0.1559 1 12] Play click audio on the keyboard
      (Audio|PlaySoundatLocation "/Game/Computer/Audio/mouse-and-keyboard-click-sounds-27527.mouse-and-keyboard-click-sounds-27527" (Transformation|GetWorldLocation (Variables|Default|GetKeyboard)) "0, 0, 0" 1.0 1.0 0.0 0 0 0 0)
      ;;[0.1559 0.1559 0.1559 1 12] Sanitize the valid key input
      (CallFunction|AddPressedKey))))

(event Custom|Released
  (params (KeyName :type String) (KeyIndex :type Integer))
  ;[1 1 1 1 34] Key Released: Sets the z-axis offset for the released key back to its default position and disables shift-hold flag
  (Utilities|RemoveKeyinLiveClicks KeyName
    (:KeyNoLongerTracked
      (CallFunction|SetKeyAnimation KeyIndex false)
      (Utilities|Time|ClearandInvalidateTimerbyHandle (Variables|Default|GetTimerHandle))
      ;;[0.1559 0.1559 0.1559 1 12] Determines the shift flag, if either shift key is holding, then shifts flag is on
      (Utilities|FlowControl|Sequence
        (:then_0
          (if (Utilities|Enum|Equal(Enum) "Left Shift" KeyName)
            (Variables|Default|SetLeftShiftHolding false)))
        (:then_1
          (if (Utilities|Enum|Equal(Enum) KeyName "Right Shift")
            (Variables|Default|SetRightShiftHolding false)))
        (:then_2
          (if (Math|Boolean|NORBoolean (Variables|Default|GetLeftShiftHolding) (Variables|Default|GetRightShiftHolding))
            (Variables|Default|SetShiftIsHeld false)))))))

(event Custom|Spam
  ;[1 1 1 1 34] Key State Change Detected: Check the key input is valid then compute pressed or released logic
  ;;[0.1559 0.1559 0.1559 1 14] Holding a key down will print it to the screen every .05 Seconds,
  (if (Variables|Default|GetKeyboardEnabled)
    (Variables|Default|SetCurrentKey (stale Custom|PressDetected _key))
    (CallFunction|AddPressedKey)))

(event Custom|Set%20WPM%20Timer
  ;[1 1 1 1 34] Key State Change Detected: Check the key input is valid then compute pressed or released logic
  ;;[0.1559 0.1559 0.1559] Sets a timer on the first key click for a task
  (Variables|Default|SetisFirstKey false)
  (Variables|Default|SetStartTimer (+ (Variables|Default|GetStartTimer) (Utilities|Time|GetRealTimeSeconds))))

(event Custom|FillTaskProgress
  (params (TaskNumber :type Integer))
  ;[1 1 1] Fills a tasks' accuracy color and sets its WPM
  (bind _fill (Timeline|Timeline PlayFromStart)
    (:Update
      (Default|FillTaskDiamonds (Variables|Default|GetComputerScreenWB) TaskNumber _fill))))

(event Custom|GlobalVarPending
  ;[1 1 1] Loops until the GlobalVariable class is loaded in, then sets the computer mesh, keyboard skeleton and enable the keyboard for user input
  (if (Variables|/Game/Globals/GlobalVariables.GlobalVariables_C|GetActorIsLoaded (Variables|Default|GetGlobalVars))
    (CallFunction|SpawnComputerType)
    (Utilities|SetObjectReferences
      (:References%20Set
        (Variables|Default|SetKeyboardEnabled true)))
    (else
      (Utilities|FlowControl|Delay 0.5)
      (CallFunction|GlobalVarPending))))

(event Custom|PressDetected
  (params (KeyName :type Text))
  ;[1 1 1 1 34] Key State Change Detected: Check the key input is valid then compute pressed or released logic
  (bind (_key _keyindex) (Utilities|CheckKeyMapandKeyboardStatus KeyName)
    (:IsValid
      (if (Variables|Default|GetisFirstKey)
        (CallFunction|SetWPMTimer))
      (bind _returnvalue (Utilities|Time|SetTimerbyEvent (delegate Custom|Spam) 0.05 true 0.5))
      (Variables|Default|SetTimerHandle _returnvalue)
      ;;[0.1559 0.1559 0.1559 1 14] Key Pressed, Sanatize for special keys and print user input to screen
      (CallFunction|Pressed _key _keyindex))))

(event Custom|ReleaseDetected
  (params (KeyName :type Text))
  ;[1 1 1 1 34] Key State Change Detected: Check the key input is valid then compute pressed or released logic
  ;;[0.1559 0.1559 0.1559 1 14] Key Released, Set key offset and clear shift flag
  (bind (_key _keyindex) (Utilities|CheckKeyMapandKeyboardStatus KeyName)
    (:IsValid
      (CallFunction|Released _key _keyindex))))

(event EventBeginPlay
  ;[1 1 1] BeginPlay: Get a ref to the class storing all of the global variables
  (bind _returnvalue (Actor|GetActorOfClass "/Game/Globals/GlobalVariables.GlobalVariables_C"))
  (Variables|Default|SetGlobalVars _returnvalue)
  (CallFunction|GlobalVarPending))

(event Input|KeyboardEvents|AnyKey
  (params (Key :type Key%20Structure :default "None"))
  (bind _returnvalue (Class|KismetInputLibrary|KeyGetDisplayName Key true))
  (bind _globalvars (Variables|Default|GetGlobalVars))
  (bind _globalvars_2 (Variables|Default|GetGlobalVars))
  (bind _isvirtualkeyboard (Variables|/Game/Globals/GlobalVariables.GlobalVariables_C|GetIsVirtualKeyboard _globalvars_2))
  (bind _slideshowactive (Variables|/Game/Globals/GlobalVariables.GlobalVariables_C|GetSlideShowActive _globalvars))
  (:Pressed
    (if _slideshowactive
      ;[1 1 1] Checks for keyboard type, used to interchange between phyiscal key input and virtual key overlap inputs
      (Default|SwitchSlides (Variables|Default|GetTaskMonitorUI) (Utilities|String|ToString(Text) _returnvalue))
      (elif (not _isvirtualkeyboard)
        (CallFunction|PressDetected _returnvalue))))
  (:Released
    (if (not _slideshowactive)
      (if (not _isvirtualkeyboard)
        (CallFunction|ReleaseDetected _returnvalue)))))

(fn ConstructionScript)

(fn SetKeyAnimation
  (params (KeyIndex :type Integer) (IsPressed :type Boolean))
  ;[1 1 1] Sets the Z-axis (Up and Down) of the specific key being pressed/released
  ;;[0.1559 0.1559 0.1559 1 12] Calls the KeyAnimation Blueprint
  (Default|UpdateKeyTranslation (Variables|Default|GetKeyAnimAB) KeyIndex (Math|Float|SelectFloat -0.35 0.0 IsPressed)))

(fn RemoveChar
  ;[1 1 1] Handles deletion of characters for both UI Widgets
  ;;[0.1559 0.1559 0.1559 1 14] Prevent indexing out of bounds
  (if (>= (Variables|Default|GetIndex) 1)
    ;;[0.1559 0.1559 0.1559 1 14] Clear the color for the char that no longer has user input
    (bind _output_get (Variables|Default|SetIndex (- (Variables|Default|GetIndex) 1)))
    (Default|DeleteCharacterColor (Variables|Default|GetTaskMonitorUI) _output_get)
    ;;[0.1559 0.1559 0.1559 1 14] Remove the last character of the stored character inputs
    (Variables|Default|SetScreenText (Utilities|String|GetSubstring (Variables|Default|GetScreenText) 0 _output_get))))

(fn AddChar
  ;[1 1 1] Tracks screen text length and inserts valid character inputs into the screen text string
  ;;[0.1559 0.1559 0.1559 1 12] Prevent non-text input from being added
  (if (not (Variables|Default|GetSpecialKeyPressed))
    ;;[0.1559 0.1559 0.1559 1 12] Increment current index, also increments Computer UI cursor
    (Variables|Default|SetIndex (+ (Variables|Default|GetIndex) 1))
    ;;[0.1559 0.1559 0.1559 1 12] Append newest character to the screens text output
    (Variables|Default|SetScreenText (Utilities|String|Append (Variables|Default|GetScreenText) (Variables|Default|GetCurrentKey)))
    (Utilities|AddClicktoClickStatTracker)))

(fn CheckNonPrintableKeys
  ;[1 1 1] Convert non-singular key names to their correct character
  (Utilities|CheckforUnusableKeys
    (:Valid%20Key
      ;;[0.1559 0.1559 0.1559 1 12] Detects backspace, delete, enter, caps, shift
      (Utilities|CheckforActionKeys
        (:NoActionKeyFound
          ;;[0.1559 0.1559 0.1559 1 12] Detects keys with symbol names
          (Utilities|CheckforSymbolKeys
            (:ValidSymbolFound
              (Variables|Default|SetCurrentKey (Variables|Default|GetSpecialChar)))))))))

(fn VerifyUserInput
  (bind _isequal (Utilities|CompareCharacters))
  (bind _globalvars (Variables|Default|GetGlobalVars))
  (bind _index (Variables|Default|GetIndex))
  (bind _returnvalue (- _index 1))
  ;[1 1 1 1 48] Checks if the user input was correct as well as handles prompt and end game transition
  ;;[0.1559 0.1559 0.1559 1 12] Prevent special keys from being compared to
  (if (Variables|Default|GetSpecialKeyPressed)
    (Variables|Default|SetSpecialKeyPressed false)
    (else
      ;;[0.1559 0.1559 0.1559 1 14] Tracks every character for valid/invalid placements
      (Utilities|Array|SetArrayElem (Variables|Default|GetCorrections) _returnvalue _isequal true)
      ;;[0.1559 0.1559 0.1559 1 12] Set the char in the prompt UI to Green/Red
      (Default|InsertCharacterColor (Variables|Default|GetTaskMonitorUI) _isequal _returnvalue)
      ;;[0.1559 0.1559 0.1559 1 14] Checks if current index is equal to the prompt length, if so handle transition
      (Variables|Default|SetCurrentKey "")
      (if (== (Variables|Default|GetIndex) (Utilities|String|Len (Default|GetPrompt (Variables|Default|GetGlobalVars))))
        ;;[0.1559 0.1559 0.1559 1 14] Clear variables and check if the last task has been complete
        (CallFunction|SetTaskStats)
        (Utilities|ClearBPVariables
          (:Variables%20reset
            (if (< (Default|GetPromptNum (Variables|Default|GetGlobalVars)) 9)
              ;;[0.1559 0.1559 0.1559 1 14] Set up the next prompt and set it to the Monitor UI
              (Default|SetNextPrompt _globalvars)
              (Default|GetNextTask (Variables|Default|GetTaskMonitorUI))
              (else
                ;;[0.1559 0.1559 0.1559 1 14] Save the tracked global variable data and disable the keyboard
                (Default|SaveUserData _globalvars)
                (Variables|Default|SetKeyboardEnabled false)))
            ;;[0.1559 0.1559 0.1559 1 14] Clears the Computer UIs stored text
            (Default|SetText (Variables|Default|GetComputerScreenWB))))))))

(fn CheckforShift
  ;[1 1 1] Convert singular key characters based on caps-lock and shift flags
  ;;[0.1559 0.1559 0.1559 1 12] Converts num to symbol if shift is held
  (Utilities|CheckforDigits
    (:NoChangeMade
      ;;[0.1559 0.1559 0.1559 1 12] ( (Caps = True AND Shift = True) OR (Caps = False AND Shift = False) ) -> Lowercase the character
      (if (== (Variables|Default|GetCapsLockOn) (Variables|Default|GetShiftIsHeld))
        (Variables|Default|SetCurrentKey (Utilities|String|ToLower (Variables|Default|GetCurrentKey)))))))

(fn AddPressedKey
  ;[1 1 1] Handles cleaning the user input, whether the key was a alphanumerical, action, or modify key
  ;;[0.1559 0.1559 0.1559 1 12] If there is more than one character, it is a non-alphanumerical key
  (Utilities|CheckforUnusableKeys
    (:Valid%20Key
      (if (> (Utilities|String|Len (Variables|Default|GetCurrentKey)) 1)
        ;;[0.1559 0.1559 0.1559 1 12] Sanitize special input
        (CallFunction|CheckNonPrintableKeys)
        (else
          ;;[0.1559 0.1559 0.1559 1 12] For upper/lower case and number/symbol conversion
          (CallFunction|CheckforShift)))
      ;;[0.1559 0.1559 0.1559 1 12] Add the char to the screen text
      (CallFunction|AddChar)
      ;;[0.1559 0.1559 0.1559 1 12] Update the screen text
      (Default|SetText (Variables|Default|GetComputerScreenWB) (Variables|Default|GetScreenText))
      ;;[0.1559 0.1559 0.1559 1 12] Compare user input to expected input
      (CallFunction|VerifyUserInput))))

(fn SetTaskStats
  (bind (_wpm _time) (Utilities|ComputeWPM))
  (bind _globalvars (Variables|Default|GetGlobalVars))
  (bind _promptnumber (Default|GetPromptNum _globalvars))
  ;[1 1 1] Computes Accuracy and WPM, then stores them to be saved post-runtime
  ;;[0.1559 0.1559 0.1559 1 14] Store tasks data for analysis after experiment
  (bind (_accuracy _incorrectchars) (Utilities|ComputeAccuracy)
    (:return
      (Default|StoreTaskStats (Variables|Default|GetGlobalVars) _wpm _time _accuracy _incorrectchars (Utilities|String|Append (Variables|Default|GetAllClickForCurrentTask) " ]"))
      ;;[0.1559 0.1559 0.1559 1 14] Set the WPM and Accuracy color to the tasks component in Computer UI
      (Default|SetTaskStats (Variables|Default|GetComputerScreenWB) _wpm _promptnumber (Math|Color|Lerp(LinearColor) "(R=1.000000,G=0.000000,B=0.000000,A=1.000000)" "(R=0.000000,G=1.000000,B=0.000000,A=1.000000)" _accuracy))
      (CallFunction|FillTaskProgress _promptnumber))))

(fn SpawnComputerType
  (bind _globalvars (Variables|Default|GetGlobalVars))
  (bind _keyboard (Variables|Default|GetKeyboard))
  (bind _computer (Variables|Default|GetComputer))
  ;[1 1 1] Spawns a specific mesh and keyboard based on the pre-set variables.
  (if (Variables|/Game/Globals/GlobalVariables.GlobalVariables_C|GetUseHP _globalvars)
    (Components|StaticMesh|SetStaticMesh _computer "/Game/Computer/Types/LabComputer/Meshes/HPKeyboard.HPKeyboard")
    (Components|SkeletalMesh|SetSkeletalMeshAsset _keyboard "/Game/Computer/Types/LabComputer/Meshes/HPKeys.HPKeys")
    ;;[0.1559 0.1559 0.1559 1 14] Adjust UI location and HP keyboard to accomadate for seperated monitor
    (Transformation|AddLocalOffset (Variables|Default|GetScreenUI) "5.500000,1.500000,3.500000" false true)
    (Transformation|AddLocalOffset (Variables|Default|GetKeyboard) "0.000000,15.000000,0.000000" false false)
    (Transformation|AddLocalOffset (Variables|Default|GetComputer) "0.000000,15.000000,0.000000" false false)
    (elif (Variables|/Game/Globals/GlobalVariables.GlobalVariables_C|GetUseBens _globalvars)
      (Components|StaticMesh|SetStaticMesh _computer "/Game/Computer/Types/BensComputer/Meshes/BensComputer-Frame.BensComputer-Frame")
      (Components|SkeletalMesh|SetSkeletalMeshAsset _keyboard "/Game/Computer/Types/BensComputer/Meshes/BenKeyboard.BenKeyboard")
      (else
        (Components|StaticMesh|SetStaticMesh _computer "/Game/Computer/Types/GeosComputer/Meshes/Computer.Computer")
        (Components|SkeletalMesh|SetSkeletalMeshAsset _keyboard "/Game/Computer/Types/GeosComputer/Meshes/Keyboard.Keyboard")))))