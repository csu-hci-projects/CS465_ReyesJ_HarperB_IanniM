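; Interactive computer with a physical keyboard that mirrors the player's typing on an on-screen widget and checks it against a target sentence.
; Each mapped key plays a click and moves that key through the KeyAnimations anim blueprint.
; Macros and lookup maps resolve shift, caps lock, symbols and deletion to build the screen text.
; Each character is compared by character code with the first SentenceBank entry, printing correct and incorrect totals.
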(event Custom|Pressed
  (params (KeyName :type String) (KeyIndex :type Integer))
  ;[1 1 1 1 34] Key Pressed: Checks that the input given is safe for manipulation and display
  (Variables|Default|SetCurrentKey KeyName)
  ;;[0.1559 0.1559 0.1559 1 12] Set the visual offset of the key on the keyboard
  (CallFunction|SetKeyAnimation KeyIndex true)
  ;;[0.1559 0.1559 0.1559 1 12] Play keyClicks on the keyboard
  (Audio|PlaySoundatLocation "/Game/PhysicalKeyboard/Audio/mouse-and-keyboard-click-sounds-27527.mouse-and-keyboard-click-sounds-27527" (Transformation|GetWorldLocation (Variables|Default|GetKeyboard)) "0, 0, 0" 1.0 1.0 0.0 0 0 0 0)
  ;;[0.1559 0.1559 0.1559 1 12] If there is more than one character, it is a non-letter/number key
  (if (> (Utilities|String|Len (Variables|Default|GetCurrentKey)) 1)
    ;;[0.1559 0.1559 0.1559 1 12] Sanitize special input
    (CallFunction|CheckNonPrintableKeys)
    (else
      ;;[0.1559 0.1559 0.1559 1 12] For upper/lower case conversion and shift+number
      (CallFunction|CheckforShift)))
  ;;[0.1559 0.1559 0.1559 1 12] Add the char to the screen text
  (CallFunction|AddChar)
  ;;[0.1559 0.1559 0.1559 1 12] Update the screen text
  (CallFunction|SetScreenText)
  ;;[0.1559 0.1559 0.1559 1 12] Compare user input to expected input
  (CallFunction|CheckSentence))

(event Custom|Released
  (params (KeyName :type String) (KeyIndex :type Integer))
  ;[1 1 1 1 34] Key Released: Sets the z-axis offset for the released key back to its default position and disables shift-hold flag
  (CallFunction|SetKeyAnimation KeyIndex false)
  (if (or (Utilities|Enum|Equal(Enum) "Left Shift" KeyName) (Utilities|Enum|Equal(Enum) KeyName "Right Shift"))
    (Variables|Default|SetShiftIsPressed false)))

(event EventBeginPlay
  ;[1 1 1] Start of program: Initialize Keyboard Anim Ref
  ;;[0.1552 0.1552 0.1552 1 14] Get the skeletal meshs (Keyboard) animation blueprint to bridge a connection for signaling when to perform clicks visually.
  (bind _askey_animations (Utilities|Casting|CastToKeyAnimations (Components|SkeletalMesh|GetAnimInstance (Variables|Default|GetKeyboard))))
  (Variables|Default|SetKeyAnimBP _askey_animations)
  ;;[0.1559 0.1559 0.1559 1 14] Small delay to prevent null refererncing
  (Utilities|FlowControl|Delay 0.1))

(event Input|KeyboardEvents|AnyKey
  (params (Key :type Key%20Structure))
  (bind _returnvalue (Class|KismetInputLibrary|KeyGetDisplayName Key true))
  (bind _keymap (Variables|Default|GetKeyMap))
  (bind _returnvalue_2 (Utilities|String|ToString(Text) _returnvalue))
  (bind (_value _returnvalue_3) (Utilities|Map|Find _keymap _returnvalue_2))
  ;[1 1 1 1 34] Key State Change Detected: Check the key input is valid then compute pressed or released logic
  (:Pressed
    (if _returnvalue_3
      ;;[0.1559 0.1559 0.1559 1 14] Key Pressed, Sanatize for special keys and print user input to screen
      (CallFunction|Pressed _returnvalue_2 _value)))
  (:Released
    (if _returnvalue_3
      ;;[0.1559 0.1559 0.1559 1 14] Key Released, Set key offset and clear shift flag
      (CallFunction|Released _returnvalue_2 _value))))

(fn ConstructionScript)

(fn SetKeyAnimation
  (params (KeyIndex :type Integer) (IsPressed :type Boolean))
  ;[1 1 1] Sets the Z-axis (Up and Down) of the specific key being pressed/released
  ;;[0.1559 0.1559 0.1559 1 12] Calls the KeyAnimation Blueprint
  (Default|UpdateKeyTranslation (Variables|Default|GetKeyAnimBP) KeyIndex (Math|Float|SelectFloat -0.35 0.0 IsPressed)))

(fn RemoveChar
  (if (>= (Variables|Default|GetIndex) 1)
    (bind _output_get (Variables|Default|SetIndex (- (Variables|Default|GetIndex) 1)))
    (Variables|Default|SetScreenText (Utilities|String|GetSubstring (Variables|Default|GetScreenText) 0 _output_get))))

(fn AddChar
  ;[1 1 1] Tracks screen text length and inserts valid character inputs into the screen text string
  ;;[0.1559 0.1559 0.1559 1 12] Prevent non-text input from being added
  (if (not (Variables|Default|GetSpecialKeyPressed))
    ;;[0.1559 0.1559 0.1559 1 12] Increment screens cursor
    (Variables|Default|SetIndex (+ (Variables|Default|GetIndex) 1))
    ;;[0.1559 0.1559 0.1559 1 12] Append newest character to the screens text output
    (Variables|Default|SetScreenText (Utilities|String|Append (Variables|Default|GetScreenText) (Variables|Default|GetCurrentKey)))))

(fn CheckNonPrintableKeys
  ;[1 1 1] Convert non-singular key names to their correct character
  ;;[0.1559 0.1559 0.1559 1 12] Detects backspace, delete, enter, caps, shift
  (Utilities|CheckforActionKeys
    (:NoActionKeyFound
      ;;[0.1559 0.1559 0.1559 1 12] Detects keys with symbol names
      (Utilities|CheckforSymbolKeys
        (:ValidSymbolFound
          (Variables|Default|SetCurrentKey (Variables|Default|GetSpecialChar)))))))

(fn SetScreenText
  ;[1 1 1] Sends the screen text stored to the UI widget that displays the screen
  (bind _ascomputer_screen (Utilities|Casting|CastToComputerScreen (UserInterface|GetWidget (Variables|Default|GetScreenUI))))
  (Default|SetText _ascomputer_screen (Variables|Default|GetScreenText)))

(fn CheckSentence
  (bind _index (Variables|Default|GetIndex))
  (bind _returnvalue (- _index 1))
  (if (Variables|Default|GetSpecialKeyPressed)
    (Variables|Default|SetSpecialKeyPressed false)
    (else
      ;[1 1 1] Tracks total corrections and messups
      (Utilities|Array|SetArrayElem (Variables|Default|GetCorrections) _returnvalue (== (Utilities|String|GetCharacterasNumber (Variables|Default|GetCurrentKey)) (Utilities|String|GetCharacterasNumber (Utilities|Array|Get(acopy) (Variables|Default|GetSentenceBank)) _returnvalue)) true)
      (if (== (Utilities|String|GetCharacterasNumber (Variables|Default|GetCurrentKey)) (Utilities|String|GetCharacterasNumber (Utilities|Array|Get(acopy) (Variables|Default|GetSentenceBank)) _returnvalue))
        (Development|PrintString "Correct!")
        (else
          (Development|PrintString "Incorrect")))
      (Variables|Default|SetCurrentKey "")
      (for _array_element (Variables|Default|GetCorrections)
        (if _array_element
          (bind _result (Math|Integer|IncrementInt (Variables|Default|GetCorrectCharacters))
            (:%20%20
              (bind _output_get (Variables|Default|SetCorrectCharacters _result))))
          (else
            (bind _result_2 (Math|Integer|IncrementInt (Variables|Default|GetIncorrectCharacters))
              (:%20%20
                (bind _output_get_2 (Variables|Default|SetIncorrectCharacters _result_2)))))))
      (Development|PrintString (Utilities|String|Append (Utilities|String|Append "Total Correct: " (Utilities|String|ToString(Integer) _output_get)) (Utilities|String|Append "                                    Total Incorrect: " (Utilities|String|ToString(Integer) _output_get_2))))
      (Variables|Default|SetCorrectCharacters 0)
      (Variables|Default|SetIncorrectCharacters 0))))

(fn CheckforShift
  ;[1 1 1] Convert singular key characters based on caps-lock and shift flags
  ;;[0.1559 0.1559 0.1559 1 12] Converts num to symbol if shift is held
  (Utilities|CheckforDigits
    (:NoChangeMade
      ;;[0.1559 0.1559 0.1559 1 12] If ( (Caps == True AND Shift == True) OR If Caps == False AND Shift == False) ) -> Lowercase the character
      (if (== (Variables|Default|GetCapsLockOn) (Variables|Default|GetShiftIsPressed))
        (Variables|Default|SetCurrentKey (Utilities|String|ToLower (Variables|Default|GetCurrentKey)))))))