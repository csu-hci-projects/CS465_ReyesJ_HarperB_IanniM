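; Computer actor with a physical keyboard that mirrors the player's typing and shows the text on a screen widget.
; Key presses are looked up in KeyMap to play a click sound and offset that key through the KeyAnimations anim instance; releases reset it.
; Named keys become symbols or deletions in a character array, which is rebuilt by prepending and reversing, then sent to the ComputerScreen widget.
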(event EventBeginPlay
  (Utilities|FlowControl|Delay 0.25)
  (bind _askey_animations (Utilities|Casting|CastToKeyAnimations (Components|SkeletalMesh|GetAnimInstance (Variables|Default|GetKeyboard))))
  (Variables|Default|SetKeyAnimBP _askey_animations)
  (Variables|Default|SetArrayOfChars (Utilities|Array|MakeArray "")))

(event Input|KeyboardEvents|AnyKey
  (params (Key :type Key%20Structure :default "None"))
  (bind _returnvalue (Class|KismetInputLibrary|KeyGetDisplayName Key true))
  (bind _returnvalue_2 (Utilities|String|ToString(Text) _returnvalue))
  (:Pressed
    (CallFunction|Pressed _returnvalue_2))
  (:Released
    (CallFunction|Released _returnvalue_2)))

(fn ConstructionScript)

(fn Pressed
  (params (KeyName :type String))
  (bind _keymap (Variables|Default|GetKeyMap))
  (bind (_value _returnvalue) (Utilities|Map|Find _keymap KeyName))
  (if _returnvalue
    (Variables|Default|SetInput KeyName)
    (Audio|PlaySoundatLocation "/Game/ProjectKeyboards/PhysicalKeyboard/Audio/mouse-and-keyboard-click-sounds-27527.mouse-and-keyboard-click-sounds-27527" (Transformation|GetWorldLocation (Variables|Default|GetKeyboard)) "0, 0, 0" 1.0 1.0 0.0 0 0 0 0)
    (CallFunction|SetNewKeyValue _value true)
    (bind _result (Math|Integer|IncrementInt (Variables|Default|GetIndex))
      (:%20%20
        (Variables|Default|SetIndex _result)
        (if (> (Utilities|String|Len (Variables|Default|GetInput)) 1)
          (CallFunction|ReplaceCommand)
          (else
            (CallFunction|AddChar (Variables|Default|GetInput))))))))

(fn Released
  (params (KeyName :type String))
  (bind _keymap (Variables|Default|GetKeyMap))
  (bind (_value _returnvalue) (Utilities|Map|Find _keymap KeyName))
  (if _returnvalue
    (CallFunction|SetNewKeyValue _value false)))

(fn SetNewKeyValue
  (params (KeyIndex :type Integer) (IsPressed :type Boolean))
  (Default|UpdateKeyTranslation (Variables|Default|GetKeyAnimBP) KeyIndex (Math|Float|SelectFloat -0.35 0.0 IsPressed)))

(fn RemoveChar
  (bind _result (Math|Integer|DecrementInt (Variables|Default|GetIndex))
    (:%20%20
      (if (!= -1 _result)
        (Utilities|Array|RemoveIndex (Variables|Default|GetArrayOfChars) (Variables|Default|GetIndex))
        (bind _result_2 (Math|Integer|DecrementInt (Variables|Default|GetIndex))
          (:%20%20
            (Variables|Default|SetIndex _result_2)
            (bind _builtstring (CallFunction|BuildString))
            (CallFunction|SetScreenText _builtstring)))))))

(fn AddChar
  (params (Char :type String))
  (Utilities|Array|Add (Variables|Default|GetArrayOfChars) Char)
  (bind _builtstring (CallFunction|BuildString))
  (Development|PrintString _builtstring)
  (CallFunction|SetScreenText _builtstring))

(fn ReplaceCommand
  (bind _input (Variables|Default|GetInput))
  (bind _input_2 (Variables|Default|GetInput))
  (if (or (Utilities|Enum|Equal(Enum) "Delete" _input_2) (Utilities|Enum|Equal(Enum) _input_2 "Backspace"))
    (CallFunction|RemoveChar)
    (else
      (CallFunction|CheckforSpecialChar _input)
      (if (Utilities|Enum|NotEqual(Enum) (Variables|Default|GetSpecialChar) _input)
        (CallFunction|AddChar (Variables|Default|GetSpecialChar))
        (Variables|Default|SetSpecialChar "")))))

(fn CheckforSpecialChar
  (params (Input :type String))
  (if (Utilities|Enum|Equal(Enum) "Equals" Input)
    (Variables|Default|SetSpecialChar "=")
    (elif (Utilities|Enum|Equal(Enum) "Hyphen" Input)
      (Variables|Default|SetSpecialChar "-")
      (elif (Utilities|Enum|Equal(Enum) "Backslash" Input)
        (Variables|Default|SetSpecialChar "\\")
        (elif (Utilities|Enum|Equal(Enum) "Right Bracket" Input)
          (Variables|Default|SetSpecialChar "]")
          (elif (Utilities|Enum|Equal(Enum) "Left Bracket" Input)
            (Variables|Default|SetSpecialChar "[")
            (elif (Utilities|Enum|Equal(Enum) "Tab" Input)
              (Variables|Default|SetSpecialChar "    ")
              (elif (Utilities|Enum|Equal(Enum) "Apostrophe" Input)
                (Variables|Default|SetSpecialChar "'")
                (elif (Utilities|Enum|Equal(Enum) "Semicolon" Input)
                  (Variables|Default|SetSpecialChar ";")
                  (elif (Utilities|Enum|Equal(Enum) "Slash" Input)
                    (Variables|Default|SetSpecialChar "/")
                    (elif (Utilities|Enum|Equal(Enum) "Space Bar" Input)
                      (Variables|Default|SetSpecialChar " ")
                      (elif (Utilities|Enum|Equal(Enum) "Period" Input)
                        (Variables|Default|SetSpecialChar ".")
                        (elif (Utilities|Enum|Equal(Enum) "Comma" Input)
                          (Variables|Default|SetSpecialChar ",")
                          (else
                            (Variables|Default|SetSpecialChar Input)))))))))))))))

(fn SetScreenText
  (params (NewText :type String))
  (bind _ascomputer_screen (Utilities|Casting|CastToComputerScreen (UserInterface|GetWidget (Variables|Default|GetScreenUI))))
  (Default|SetText _ascomputer_screen NewText)
  (Variables|Default|SetSentence ""))

(fn BuildString
  (for _array_element (Variables|Default|GetArrayOfChars)
    (Variables|Default|SetSentence (Utilities|String|Append _array_element (Variables|Default|GetSentence))))
  (return (Utilities|String|Reverse (Variables|Default|GetSentence))))