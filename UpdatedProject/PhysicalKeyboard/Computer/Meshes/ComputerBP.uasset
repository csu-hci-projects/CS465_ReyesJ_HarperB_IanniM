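; Computer actor that runs a typing test, mirroring real key presses on an animated keyboard mesh and its screen widget.
; Mapped keys move through the KeyAnimations anim Blueprint with a click sound, while a looping timer repeats input.
; Input resolves Shift, Caps Lock, symbols and deletes into screen text, checked per character against the current SentenceBank task.
; Completed tasks send WPM and accuracy color to ComputerScreen, animate progress and load the next sentence.
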(event Custom|Pressed
  (params (KeyName :type String) (KeyIndex :type Integer))
  ;[1 1 1 1 34] Key Pressed: Checks that the input given is safe for manipulation and display
  (bind _output_get (Variables|Default|SetCurrentKey KeyName))
  (Utilities|InsertKeyinLiveClicks _output_get
    (:TrackingKey
      ;;[0.1559 0.1559 0.1559 1 12] Set the visual offset of the key on the keyboard
      (CallFunction|SetKeyAnimation KeyIndex true)
      ;;[0.1559 0.1559 0.1559 1 12] Play keyClicks on the keyboard
      (Audio|PlaySoundatLocation "/Game/PhysicalKeyboard/Audio/mouse-and-keyboard-click-sounds-27527.mouse-and-keyboard-click-sounds-27527" (Transformation|GetWorldLocation (Variables|Default|GetKeyboard)) "0, 0, 0" 1.0 1.0 0.0 0 0 0 0)
      (CallFunction|AddPressedKey))))

(event Custom|Released
  (params (KeyName :type String) (KeyIndex :type Integer))
  ;[1 1 1 1 34] Key Released: Sets the z-axis offset for the released key back to its default position and disables shift-hold flag
  (Utilities|RemoveKeyinLiveClicks KeyName
    (:KeyNoLongerTracked
      (CallFunction|SetKeyAnimation KeyIndex false)
      (Utilities|Time|ClearandInvalidateTimerbyHandle (Variables|Default|GetTimerHandle))
      (if (or (Utilities|Enum|Equal(Enum) "Left Shift" KeyName) (Utilities|Enum|Equal(Enum) KeyName "Right Shift"))
        (Variables|Default|SetShiftIsPressed false)))))

(event Custom|Spam
  ;[1 1 1 1 34] Key State Change Detected: Check the key input is valid then compute pressed or released logic
  (Variables|Default|SetCurrentKey (stale Input|KeyboardEvents|AnyKey _key))
  (CallFunction|AddPressedKey))

(event Custom|Set%20WPM%20Timer
  ;[1 1 1 1 34] Key State Change Detected: Check the key input is valid then compute pressed or released logic
  ;;[1 1 1] Sets a timer on the first key click for a task
  (Variables|Default|SetisFirstKey false)
  (Variables|Default|SetStartTimer (+ (Variables|Default|GetStartTimer) (Utilities|Time|GetRealTimeSeconds))))

(event Custom|FillTaskProgress
  (params (TaskNumber :type Integer))
  ;[1 1 1] Calls the Screen UI to fill a finished tasks ui node
  (bind _fill (Timeline|Timeline PlayFromStart)
    (:Update
      (Default|FillTaskDiamonds (Variables|Default|GetComputerScreenWB) TaskNumber _fill))))

(event EventBeginPlay
  ;[1 1 1] Start of program: Initialize Keyboard Anim Ref
  ;;[0.1552 0.1552 0.1552 1 14] Get the skeletal meshs (Keyboard) animation blueprint to bridge a connection for signaling when to perform clicks visually.
  (bind _askey_animations (Utilities|Casting|CastToKeyAnimations (Components|SkeletalMesh|GetAnimInstance (Variables|Default|GetKeyboard))))
  (Variables|Default|SetKeyAnimAB _askey_animations)
  (bind _ascomputer_screen (Utilities|Casting|CastToComputerScreen (UserInterface|GetWidget (Variables|Default|GetScreenUI))))
  (Variables|Default|SetComputerScreenWB _ascomputer_screen)
  (Variables|Default|SetCurrentTask (.Value (Utilities|Map|Find (Variables|Default|GetSentenceBank) (Variables|Default|GetTaskNumber))))
  ;;[0.1559 0.1559 0.1559 1 14] Small delay to prevent null refrencing
  (Utilities|FlowControl|Delay 0.1)
  (Variables|Default|SetKeyboardEnabled true))

(event Input|KeyboardEvents|AnyKey
  (params (Key :type Key%20Structure :default "None"))
  (bind _returnvalue (Class|KismetInputLibrary|KeyGetDisplayName Key true))
  ;[1 1 1 1 34] Key State Change Detected: Check the key input is valid then compute pressed or released logic
  (:Pressed
    (bind (_key _keyindex) (Utilities|CheckKeyMapandKeyboardStatus _returnvalue)
      (:IsValid
        (if (Variables|Default|GetisFirstKey)
          (CallFunction|SetWPMTimer))
        (bind _returnvalue_2 (Utilities|Time|SetTimerbyEvent (delegate Custom|Spam) 0.05 true 0.5))
        (Variables|Default|SetTimerHandle _returnvalue_2)
        ;;[0.1559 0.1559 0.1559 1 14] Key Pressed, Sanatize for special keys and print user input to screen
        (CallFunction|Pressed _key _keyindex))))
  (:Released
    (bind (_key_2 _keyindex_2) (Utilities|CheckKeyMapandKeyboardStatus _returnvalue)
      (:IsValid
        ;;[0.1559 0.1559 0.1559 1 14] Key Released, Set key offset and clear shift flag
        (CallFunction|Released _key_2 _keyindex_2)))))

(fn ConstructionScript)

(fn SetKeyAnimation
  (params (KeyIndex :type Integer) (IsPressed :type Boolean))
  ;[1 1 1] Sets the Z-axis (Up and Down) of the specific key being pressed/released
  ;;[0.1559 0.1559 0.1559 1 12] Calls the KeyAnimation Blueprint
  (Default|UpdateKeyTranslation (Variables|Default|GetKeyAnimAB) KeyIndex (Math|Float|SelectFloat -0.35 0.0 IsPressed)))

(fn RemoveChar
  (if (>= (Variables|Default|GetIndex) 1)
    (bind _output_get (Variables|Default|SetIndex (- (Variables|Default|GetIndex) 1)))
    (Variables|Default|SetScreenText (Utilities|String|GetSubstring (Variables|Default|GetScreenText) 0 _output_get))))

(fn AddChar
  ;[1 1 1] Tracks screen text length and inserts valid character inputs into the screen text string
  ;;[0.1559 0.1559 0.1559 1 12] Prevent non-text input from being added
  (if (not (Variables|Default|GetSpecialKeyPressed))
    ;;[0.1559 0.1559 0.1559 1 12] Increment screens cursor
    (Variables|Default|SetIndex (+ (Variables|Default|GetIndex) 1))
    ;;[0.1559 0.1559 0.1559 1 12] Append newest character to the screens text output
    (Variables|Default|SetScreenText (Utilities|String|Append (Variables|Default|GetScreenText) (Variables|Default|GetCurrentKey)))))

(fn CheckNonPrintableKeys
  ;[1 1 1] Convert non-singular key names to their correct character
  ;;[0.1559 0.1559 0.1559 1 12] Detects backspace, delete, enter, caps, shift
  (Utilities|CheckforActionKeys
    (:NoActionKeyFound
      ;;[0.1559 0.1559 0.1559 1 12] Detects keys with symbol names
      (Utilities|CheckforSymbolKeys
        (:ValidSymbolFound
          (Variables|Default|SetCurrentKey (Variables|Default|GetSpecialChar)))))))

(fn SetScreenText
  ;[1 1 1] Sends the screen text stored to the UI widget that displays the screen
  (Default|SetText (Variables|Default|GetComputerScreenWB) (Variables|Default|GetScreenText)))

(fn CheckSentence
  (bind _index (Variables|Default|GetIndex))
  (bind _returnvalue (- _index 1))
  (if (Variables|Default|GetSpecialKeyPressed)
    (Variables|Default|SetSpecialKeyPressed false)
    (else
      ;[1 1 1] Tracks every character for valid/invalid placements
      (Utilities|Array|SetArrayElem (Variables|Default|GetCorrections) _returnvalue (== (Utilities|String|GetCharacterasNumber (Variables|Default|GetCurrentTask) _returnvalue) (Utilities|String|GetCharacterasNumber (Variables|Default|GetCurrentKey))) true)
      (Variables|Default|SetCurrentKey "")
      (if (== (Utilities|Array|Length (Variables|Default|GetCorrections)) (Utilities|String|Len (Variables|Default|GetCurrentTask)))
        (CallFunction|SetTaskStats)
        (bind _result (Math|Integer|IncrementInt (Variables|Default|GetTaskNumber))
          (:%20%20
            (bind _output_get (Variables|Default|SetTaskNumber _result))
            (Variables|Default|SetCurrentTask (.Value (Utilities|Map|Find (Variables|Default|GetSentenceBank) _output_get)))
            (Utilities|ClearBPVariables
              (:Variables%20reset
                (CallFunction|SetScreenText)))))))))

(fn CheckforShift
  ;[1 1 1] Convert singular key characters based on caps-lock and shift flags
  ;;[0.1559 0.1559 0.1559 1 12] Converts num to symbol if shift is held
  (Utilities|CheckforDigits
    (:NoChangeMade
      ;;[0.1559 0.1559 0.1559 1 12] If ( (Caps == True AND Shift == True) OR If Caps == False AND Shift == False) ) -> Lowercase the character
      (if (== (Variables|Default|GetCapsLockOn) (Variables|Default|GetShiftIsPressed))
        (Variables|Default|SetCurrentKey (Utilities|String|ToLower (Variables|Default|GetCurrentKey)))))))

(fn AddPressedKey
  ;[0.1559 0.1559 0.1559 1 12] If there is more than one character, it is a non-letter/number key
  (Utilities|CheckforUnusableKeys
    (:Valid%20Key
      (if (> (Utilities|String|Len (Variables|Default|GetCurrentKey)) 1)
        ;[0.1559 0.1559 0.1559 1 12] Sanitize special input
        (CallFunction|CheckNonPrintableKeys)
        (else
          ;[0.1559 0.1559 0.1559 1 12] For upper/lower case conversion and shift+number
          (CallFunction|CheckforShift)))
      ;[0.1559 0.1559 0.1559 1 12] Add the char to the screen text
      (CallFunction|AddChar)
      ;[0.1559 0.1559 0.1559 1 12] Update the screen text
      (CallFunction|SetScreenText)
      ;[0.1559 0.1559 0.1559 1 12] Compare user input to expected input
      (CallFunction|CheckSentence))))

(fn SetTaskStats
  (bind _tasknumber (Variables|Default|GetTaskNumber))
  (bind _accuracy (Utilities|ComputeAccuracy)
    (:return
      (bind _wpm (Utilities|ComputeWPM)
        (:return
          (Default|SetTaskStats (Variables|Default|GetComputerScreenWB) _wpm _tasknumber (Math|Color|Lerp(LinearColor) "(R=1.000000,G=0.000000,B=0.000000,A=1.000000)" "(R=0.000000,G=1.000000,B=0.000000,A=1.000000)" _accuracy))
          (CallFunction|FillTaskProgress _tasknumber))))))