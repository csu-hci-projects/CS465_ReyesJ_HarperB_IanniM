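; Test room actor that powers up its ceiling light panels and front conveyor belt when play begins in user mode.
; BeginPlay checks the user mode flag on the GlobalVariables actor, then a timeline drives the panels' Opacity parameter.
; After a short delay, it sets the belt material's PannerSpeed to fake movement.
; The construction script creates the belt's dynamic material instance, and GetLightPanels exposes the panels.
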(event EventBeginPlay
  ;[1 1 1] Gets a reference to the global variable BP and then checks if user mode is preset, if so play timeline to turn on the ceiling panel lights
  (bind _returnvalue (Actor|GetActorOfClass "/Game/Globals/GlobalVariables.GlobalVariables_C"))
  (bind _output_get (Variables|Default|SetGlobalVar _returnvalue))
  (bind _isusermode (Default|GetIsUserMode _output_get))
  (if _isusermode
    (bind _lightturningon (Timeline|Timeline Play)
      (:Update
        (Rendering|Material|SetScalarParameterValueonMaterials (Variables|Default|GetLightPanels) "Opacity" _lightturningon))
      (:Finished
        (Utilities|FlowControl|Delay 2.0)
        ;;[0.1559 0.1559 0.1559 1 14] Moves the conveyor belts material on its y-axis to make it look like its actually moving
        (Rendering|Material|SetVectorParameterValueonMaterials (Variables|Default|GetConveyorBeltFront) "PannerSpeed" "0.000000,0.050000,0.000000")))))

(event Collision|EventActorBeginOverlap
  (params (OtherActor :type Actor%20Object%20Reference)))

(event EventTick
  (params (DeltaSeconds :type Float%20%28single-precision%29)))

(fn ConstructionScript
  (bind _returnvalue (Rendering|Material|CreateDynamicMaterialInstance (Variables|Default|GetConveyorBeltFront) 0 "/Game/BlenderImports/TestRoom/Conveyor/Material/ConveyorBelts_Baked.ConveyorBelts_Baked" "None" :!class /Script/Engine.PrimitiveComponent))
  (bind _output_get (Variables|Default|SetMaterialInstance _returnvalue))
  (Rendering|Material|SetMaterial (Variables|Default|GetConveyorBeltFront) 0 _output_get))

(fn GetLightPanels
  (return (Variables|Default|GetLightPanels)))